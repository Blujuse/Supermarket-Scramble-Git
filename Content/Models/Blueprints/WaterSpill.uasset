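; WaterSpill is a placeable hazard that makes the player slide.
; Overlapping SlippyZone removes ground friction and lowers walking braking deceleration on PlayerBP's CharacterMovement.
; Leaving the zone restores hard-coded values after a ten-second delay, with no check for re-entry.
; The construction script toggles the plane's visibility and scales the plane and zone horizontally by a shared Size.
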(event `self.SlippyZone.OnComponentBeginOverlap`
  (params (OverlappedComponent :type "PrimitiveComponent Object Reference") (OtherActor :type "Actor Object Reference") (OtherComp :type "PrimitiveComponent Object Reference") (OtherBodyIndex :type Integer) (bFromSweep :type Boolean) (SweepResult :type "HitResult Structure (by ref)"))
  (bind _asplayer_bp (cast `/Game/Characters/PlayerBP` OtherActor))
  (bind _charactermovement (`Character.CharacterMovement` _asplayer_bp))
  (set `CharacterMovementComponent.GroundFriction` 0.0 _charactermovement)
  (set `CharacterMovementComponent.BrakingDecelerationWalking` 350.0 _charactermovement)
  (`KismetSystemLibrary.PrintString` "Slippy"))

(event `self.SlippyZone.OnComponentEndOverlap`
  (params (OverlappedComponent :type "PrimitiveComponent Object Reference") (OtherActor :type "Actor Object Reference") (OtherComp :type "PrimitiveComponent Object Reference") (OtherBodyIndex :type Integer))
  (bind _asplayer_bp (cast `/Game/Characters/PlayerBP` OtherActor))
  (`KismetSystemLibrary.Delay` 10.0)
  (`KismetSystemLibrary.PrintString` "No Slippy")
  (bind _charactermovement (`Character.CharacterMovement` _asplayer_bp))
  (set `CharacterMovementComponent.GroundFriction` 8.0 _charactermovement)
  (set `CharacterMovementComponent.BrakingDecelerationWalking` 2000.0 _charactermovement))

(fn `UserConstructionScript`
  (bind _size (`self.Size`))
  (`SceneComponent.SetVisibility` (`self.Plane`) (`self.ShowPlane?`) false)
  (`SceneComponent.SetRelativeScale3D` (`self.Plane`) (`KismetMathLibrary.MakeVector` _size _size 1.0))
  (`SceneComponent.SetRelativeScale3D` (`self.SlippyZone`) (`KismetMathLibrary.MakeVector` _size _size 1.0)))