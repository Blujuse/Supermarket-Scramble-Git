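; Milk collectable actor that the player picks up by walking into its box collision.
; On overlap with the player pawn, it sets the MilkCollected flag on PlayerBP.
; It then shrinks its mesh to zero scale in one step, spawns an Item_Explosion Niagara effect at the mesh location and destroys itself after a very short delay.
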(event `self.BoxCol.OnComponentBeginOverlap`
  (params (OverlappedComponent :type "PrimitiveComponent Object Reference") (OtherActor :type "Actor Object Reference") (OtherComp :type "PrimitiveComponent Object Reference") (OtherBodyIndex :type Integer) (bFromSweep :type Boolean) (SweepResult :type "HitResult Structure (by ref)"))
  (if (== OtherActor (`GameplayStatics.GetPlayerPawn` 0))
    (bind _asplayer_bp (cast `/Game/Blueprints/Player/PlayerBP` (`GameplayStatics.GetPlayerCharacter` 0)))
    (set `/Game/Blueprints/Player/PlayerBP.MilkCollected` true _asplayer_bp)
    (`SceneComponent.SetWorldScale3D` (`self.StaticMesh`) (`KismetMathLibrary.VLerp` (`SceneComponent.K2_GetComponentScale` (`self.StaticMesh`)) (0.0 0.0 0.0) 1.0))
    (bind _returnvalue (`NiagaraFunctionLibrary.SpawnSystemAtLocation` "/Game/Particles/Item_Explosion.Item_Explosion" (`SceneComponent.K2_GetComponentLocation` (`self.StaticMesh`))))
    (set `self.Niagara` _returnvalue)
    (`KismetSystemLibrary.Delay` 0.01)
    (`self.K2_DestroyActor`)))

(fn `UserConstructionScript`)